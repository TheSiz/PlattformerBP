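; BP_Obstacle is a moving environment obstacle that travels in a straight line from its StartingPoint toward its EndingPoint.
; BeginPlay caches both world positions, and Tick moves the actor without sweep at MovementSpeed.
; SetJourneyDistance measures progress, and SetMovementDirection supplies the normalized direction.
; The endpoint swap for reversing is only partly wired: the target update never runs, so no return trip occurs.
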(event `self.ReceiveBeginPlay`
  (bind _output_get (set `self.InitialStartLocation` (`SceneComponent.K2_GetComponentLocation` (`self.StartingPoint`))))
  (set `self.Location` _output_get)
  (set `self.InitialTargetLocation` (`SceneComponent.K2_GetComponentLocation` (`self.EndingPoint`)))
  (set `self.MovementSpeed` (`self.MovementSpeed`)))

(event `self.ReceiveTick`
  (params (DeltaSeconds :type "Float (single-precision)"))
  (`self.SetJourneyDistance`)
  (bind _movedirection (`self.SetMovementDirection`))
  (set `self.Location` (+ (`self.Location`) (* _movedirection (* DeltaSeconds (`self.MovementSpeed`)))))
  (`self.K2_SetActorLocation` (`self.Location`)))

(fn `SetJourneyDistance`
  (set `self.Location` (`self.K2_GetActorLocation` self))
  (set `self.JourneyLength` (`KismetMathLibrary.VSize` (- (`self.InitialTargetLocation`) (`self.InitialStartLocation`))))
  (set `self.JourneyTraveled` (`KismetMathLibrary.VSize` (- (`self.Location`) (`self.InitialStartLocation`))))
  (return))

(fn `SetMovementDirection`
  (returns (MoveDirection :type "Vector Structure"))
  (locals (MoveDirectionLocal :type "Vector Structure") (SwapLocal :type "Vector Structure"))
  (if (>= (`self.JourneyTraveled`) (`self.JourneyLength`))
    (set `local.SwapLocal` (`self.InitialStartLocation`))
    (set `self.InitialStartLocation` (`self.InitialTargetLocation`))
    (else
      (bind _output_get (set `local.MoveDirectionLocal` (`KismetMathLibrary.Normal` (- (`self.InitialTargetLocation`) (`self.InitialStartLocation`)))))
      (return _output_get))))

(fn `UserConstructionScript`)